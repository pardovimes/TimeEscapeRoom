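; Game state that spawns a clone pawn which replays the player's recorded movement from the previous countdown cycle.
; A looping one-second timer samples the player pawn's transform into an auxiliary array, copies it to the playback array when the countdown expires, then clears the buffer.
; The countdown also selects the playback index, and a timeline lerps the clone toward that transform to smooth movement between samples.
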(event `Counter`
  (bind _countdown (`self.CountDown`))
  (if (<= _countdown 0.0)
    (set `self.CountDown` 10.0)
    (else
      (set `self.CountDown` (- _countdown 1.0)))))

(event `ArrayManager`
  (bind _pawntansformsaux (`self.PawnTansformsAux`))
  (`KismetArrayLibrary.Array_Add` _pawntansformsaux (`self.GetTransform` (`GameplayStatics.GetPlayerPawn` 0)))
  (if (<= (`self.CountDown`) 0.0)
    (set `self.PawnTansforms` _pawntansformsaux)
    (`KismetArrayLibrary.Array_Clear` _pawntansformsaux)))

(event `self.ReceiveBeginPlay`
  (`KismetSystemLibrary.K2_SetTimer` null "TimerCount" 1.0 true)
  (`self.ArrayManager`))

(event `TimerCount`
  (`|ExecutionSequence`
    (:`then_0`
      (`self.ArrayManager`))
    (:`then_1`
      (`self.MoveClonedPawn`))
    (:`then_2`
      (`self.Counter`))))

(event `MoveClonedPawn`
  (bind _pawntansforms (`self.PawnTansforms`))
  (bind _clonedpawn (`self.ClonedPawn`))
  (if (!= (`KismetArrayLibrary.Array_Length` (`self.PawnTansforms`)) 0)
    (`/Engine/EditorBlueprintResources/StandardMacros.IsValid` (`self.ClonedPawn`)
      (:`Is Valid`
        (bind (_direction _move) (`Timeline|MovingClonedPawn` :!via `PlayFromStart` :!label _label)
          (:`Update`
            (`self.K2_SetActorTransform` _clonedpawn (`KismetMathLibrary.TLerp` (`self.GetTransform` _clonedpawn) (`KismetArrayLibrary.Array_Get` _pawntansforms (`KismetMathLibrary.FTrunc` (`KismetMathLibrary.Abs` (- (`self.CountDown`) (`KismetMathLibrary.Conv_IntToDouble` (- (`KismetArrayLibrary.Array_Length` _pawntansforms) 1)))))) _move) false false))))
      (:`Is Not Valid`
        (bind _returnvalue (`|SpawnActorFromClass` "/Game/DefaultPawn_BP.DefaultPawn_BP_C" (`KismetArrayLibrary.Array_Get` _pawntansforms) "Undefined" "OverrideRootScale"))
        (set `self.ClonedPawn` _returnvalue)
        (goto _label :!via `PlayFromStart`)))))

(fn `UserConstructionScript`)